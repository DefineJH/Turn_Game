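; BP_Light feeds a directional light's state into the MP_LightParam material parameter collection so materials can read it.
; It writes the inverted forward vector as SunLightDir, along with the light color as LightColor and intensity as LightInten.
; The same writes run in the Construction Script for in-editor updates and on every Tick at runtime.
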(event `self.ReceiveTick`
  (params (DeltaSeconds :type "Float (single-precision)"))
  (bind _directionallight (`self.DirectionalLight`))
  (`KismetMaterialLibrary.SetVectorParameterValue` "/Game/Misc/MP_LightParam.MP_LightParam" "SunLightDir" (`KismetMathLibrary.Conv_VectorToLinearColor` (* (`SceneComponent.GetForwardVector` _directionallight) -1)))
  (`KismetMaterialLibrary.SetVectorParameterValue` "/Game/Misc/MP_LightParam.MP_LightParam" "LightColor" (`LightComponentBase.GetLightColor` _directionallight))
  (`KismetMaterialLibrary.SetScalarParameterValue` "/Game/Misc/MP_LightParam.MP_LightParam" "LightInten" (`LightComponentBase.Intensity` _directionallight)))

(fn `UserConstructionScript`
  (bind _directionallight (`self.DirectionalLight`))
  (`KismetMaterialLibrary.SetVectorParameterValue` "/Game/Misc/MP_LightParam.MP_LightParam" "SunLightDir" (`KismetMathLibrary.Conv_VectorToLinearColor` (* (`SceneComponent.GetForwardVector` _directionallight) -1)))
  (`KismetMaterialLibrary.SetVectorParameterValue` "/Game/Misc/MP_LightParam.MP_LightParam" "LightColor" (`LightComponentBase.GetLightColor` _directionallight))
  (`KismetMaterialLibrary.SetScalarParameterValue` "/Game/Misc/MP_LightParam.MP_LightParam" "LightInten" (`LightComponentBase.Intensity` _directionallight)))