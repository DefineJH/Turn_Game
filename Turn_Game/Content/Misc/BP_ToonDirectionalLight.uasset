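; Directional light Blueprint that feeds its lighting data to materials, apparently for toon shading.
; It writes the negated forward vector, color and intensity of its light component into the MP_LightParam Material Parameter Collection.
; The Construction Script and Tick repeat the same writes, so the parameters update on construction and every frame at runtime.
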(event `self.ReceiveTick`
  (params (DeltaSeconds :type "Float (single-precision)"))
  (bind _lightcomponent (`self.LightComponent`))
  (`KismetMaterialLibrary.SetVectorParameterValue` "/Game/Misc/MP_LightParam.MP_LightParam" "SunLightDir" (`KismetMathLibrary.Conv_VectorToLinearColor` (* (`SceneComponent.GetForwardVector` _lightcomponent) -1)))
  (`KismetMaterialLibrary.SetVectorParameterValue` "/Game/Misc/MP_LightParam.MP_LightParam" "LightColor" (`LightComponentBase.GetLightColor` _lightcomponent))
  (`KismetMaterialLibrary.SetScalarParameterValue` "/Game/Misc/MP_LightParam.MP_LightParam" "LightInten" (`LightComponentBase.Intensity` _lightcomponent)))

(fn `UserConstructionScript`
  (bind _lightcomponent (`self.LightComponent`))
  (`KismetMaterialLibrary.SetVectorParameterValue` "/Game/Misc/MP_LightParam.MP_LightParam" "SunLightDir" (`KismetMathLibrary.Conv_VectorToLinearColor` (* (`SceneComponent.GetForwardVector` _lightcomponent) -1)))
  (`KismetMaterialLibrary.SetVectorParameterValue` "/Game/Misc/MP_LightParam.MP_LightParam" "LightColor" (`LightComponentBase.GetLightColor` _lightcomponent))
  (`KismetMaterialLibrary.SetScalarParameterValue` "/Game/Misc/MP_LightParam.MP_LightParam" "LightInten" (`LightComponentBase.Intensity` _lightcomponent)))